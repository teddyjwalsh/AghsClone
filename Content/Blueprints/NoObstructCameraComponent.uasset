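; NoObstructCameraComponent is a scene component that makes terrain transparent when it hides a Hero from view.
; Each Tick it first resets every SceneTerrain actor to opaque.
; It then line-traces static and dynamic world objects from its own location to each Hero, setting a blocking SceneTerrain hit to transparent.
; Each trace reveals only the first blocker, and the camera manager location lookup is unused.
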(event EventBeginPlay)

(event EventTick
  (params (DeltaSeconds :type Float%20%28single-precision%29))
  (bind _outactors (Actor|GetAllActorsOfClass "/Game/Blueprints/SceneTerrain.SceneTerrain_C"))
  (for _array_element _outactors
    (Default|SetTransparent _array_element false))
  (bind _outactors_2 (Actor|GetAllActorsOfClass "/Script/AghsClone.Hero"))
  (for _array_element_2 _outactors_2
    (bind _outhit (Collision|LineTraceForObjects (Transformation|GetWorldLocation) (Transformation|GetActorLocation _array_element_2) (Utilities|Array|MakeArray "ObjectTypeQuery1" "ObjectTypeQuery2") false 0 "None"))
    (if (and (.bBlockingHit (Collision|BreakHitResult _outhit)) (!= (.HitActor (Collision|BreakHitResult _outhit)) _array_element_2))
      (bind _asscene_terrain (Utilities|Casting|CastToSceneTerrain (.HitActor (Collision|BreakHitResult _outhit))))
      (Default|SetTransparent _asscene_terrain true))))